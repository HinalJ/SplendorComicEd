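; CardGamePawn is the pawn for the card game, which creates the hand and handles pause menu input.
; On BeginPlay, MakeHand spawns a Hand actor, stores it and attaches it to HandAttachPoint.
; F10 toggles game pause and the CardGameHUD pause menu, playing its blur-fade animation forward to show it.
; On unpause, the animation plays in reverse and a short delay precedes hiding the menu.
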(event `self.ReceiveBeginPlay`
  (`self.MakeHand`))

(event `Key|F10` :paused true
  (params (Key :type "Key Structure"))
  (:`Pressed`
    (bind _ascard_game_hud (cast `/Game/CardGameTemplate/Blueprints/CardGameHUD` (`PlayerController.GetHUD` (`GameplayStatics.GetPlayerController` 0))))
    (if (`GameplayStatics.IsGamePaused`)
      (`GameplayStatics.SetGamePaused` false)
      (bind _pausemenu (`/Game/CardGameTemplate/Blueprints/CardGameHUD.PauseMenu` _ascard_game_hud))
      (`UserWidget.PlayAnimation` _pausemenu (`/Game/CardGameTemplate/Blueprints/TopDownPauseUI.BlurFadeAnimation` _pausemenu) 0.0 1 "Reverse" 1.0 false)
      (`KismetSystemLibrary.Delay` 0.2)
      (`Widget.SetVisibility` _pausemenu "Hidden")
      (else
        (`Widget.SetVisibility` _pausemenu "Visible")
        (`GameplayStatics.SetGamePaused` true)
        (`UserWidget.PlayAnimation` _pausemenu (`/Game/CardGameTemplate/Blueprints/TopDownPauseUI.BlurFadeAnimation` _pausemenu) 0.0 1 "Forward" 1.0 false)))))

(fn `MakeHand`
  (bind _returnvalue (`|SpawnActorFromClass` "/Game/CardGameTemplate/Blueprints/Hand.Hand_C" (`KismetMathLibrary.MakeTransform` (0.0 0.0 0.0)) "Undefined" "OverrideRootScale" null null))
  (bind _output_get (set `self.Hand` _returnvalue))
  (`self.K2_AttachToComponent` _output_get (`self.HandAttachPoint`) "None" "KeepRelative" "KeepRelative" "KeepRelative" true))

(fn `UserConstructionScript`)