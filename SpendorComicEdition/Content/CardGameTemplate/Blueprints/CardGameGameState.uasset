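; Game state for a card game template that passes control between player pawns in hot-seat fashion on a single local controller.
; On BeginPlay it gathers every CardGamePawn in the level and has player controller 0 possess the first one.
; AdvanceTurnPlayer increments the turn index, wrapping at the player count, then unpossesses and repossesses that controller onto the next pawn.
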(event `self.ReceiveBeginPlay`
  (bind _outactors (`GameplayStatics.GetAllActorsOfClass` "/Game/CardGameTemplate/Blueprints/CardGamePawn.CardGamePawn_C"))
  (bind _output_get (set `self.PlayerPawns` _outactors))
  (`Controller.Possess` (`GameplayStatics.GetPlayerController` 0) (`|GetArrayItem` _output_get)))

(fn `AdvanceTurnPlayer`
  (bind _returnvalue (+ (`self.TurnPlayer`) 1))
  (set `self.TurnPlayer` (select `bool` (== _returnvalue (`self.NumPlayers`)) :`false` _returnvalue))
  (`Controller.UnPossess` (`GameplayStatics.GetPlayerController` 0))
  (`Controller.Possess` (`GameplayStatics.GetPlayerController` 0) (`|GetArrayItem` (`self.PlayerPawns`) (`self.TurnPlayer`))))

(fn `UserConstructionScript`)